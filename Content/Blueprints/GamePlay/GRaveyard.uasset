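; Card game graveyard pile that records a player's discarded cards and shows them as a stack.
; On the server it stores card names and data structs from a card actor or name lookup, trimming older actors so the top card shows.
; Removing a card by index clears the displayed actor and respawns the top card from stored data through the player's controller.
; A separate visual event hides or raises the stack mesh according to card count.
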(event `self.ReceiveBeginPlay`
  ;[1 0 0.09375] On Begin hide deck model
  (`SceneComponent.SetHiddenInGame` (`self.SM_Graveyard`) true false))

(event `AddToGraveyard`
  (params (EnteringCard :type "/Game/Blueprints/GamePlay/Locam_3DCard Object Reference") (OrByName :type Name))
  ;[1 0 0.2578] Add Card To Graveyard
  (`/Engine/EditorBlueprintResources/ActorMacros.Switch Has Authority`
    (:`Authority`
      (`/Engine/EditorBlueprintResources/StandardMacros.IsValid` EnteringCard
        (:`Is Valid`
          (`KismetArrayLibrary.Array_AddUnique` (`self.ActorsInGraveyard`) EnteringCard)
          (`KismetArrayLibrary.Array_Add` (`self.GraveyardList`) (`/Game/Blueprints/GamePlay/Locam_3DCard.CardDataTableName` EnteringCard))
          (`KismetArrayLibrary.Array_Add` (`self.GraveyardStructList`) (`/Game/Blueprints/GamePlay/Locam_3DCard.CardAttibutes` EnteringCard)))
        (:`Is Not Valid`
          (bind _cardstruct (`/Game/Blueprints/Library/BP_Deck_flib.GetCardData` OrByName))
          (`KismetArrayLibrary.Array_Add` (`self.GraveyardList`) OrByName)
          (`KismetArrayLibrary.Array_Add` (`self.GraveyardStructList`) _cardstruct)))
      (`self.HideUnseenCardsInGraveyard`))))

(event `AddToGraeyardVisual`
  ;[1 0 0.2578] Add Card To Graveyard
  (`self.ScaleCardGraveyardStaticMesh`))

(event `Event_RemoveCardFromGraveyard`
  (params (Card :type Name) (Index :type Integer))
  (`/Engine/EditorBlueprintResources/ActorMacros.Switch Has Authority`
    (:`Authority`
      (`self.RemoveCardFromGraveyard` Card Index)
      (`self.RecreateTopGraveyardCardActor`))))

(fn `GetCardInGraveyardLocation`
  (params (add :type Integer))
  (returns (ReturnValue :type "Vector Structure"))
  (bind (_returnvalue_x _returnvalue_y _returnvalue_z) (`KismetMathLibrary.BreakVector` (`self.K2_GetActorLocation` self)))
  (return (`KismetMathLibrary.MakeVector` _returnvalue_x _returnvalue_y (+ _returnvalue_z (+ (* 1.5 (`KismetMathLibrary.Conv_IntToDouble` (+ add (`KismetArrayLibrary.Array_Length` (`self.GraveyardList`))))) 10.0)))))

(fn `HideUnseenCardsInGraveyard`
  (bind _actorsingraveyard (`self.ActorsInGraveyard`))
  (if (> (`KismetArrayLibrary.Array_Length` _actorsingraveyard) 1)
    (for (_array_element _array_index) _actorsingraveyard
      (`/Engine/EditorBlueprintResources/StandardMacros.IsValid` _array_element
        (:`Is Valid`
          (if (not (== _array_index (`KismetArrayLibrary.Array_LastIndex` _actorsingraveyard)))
            (`/Game/Blueprints/GamePlay/Locam_3DCard.RemoveCardActor` _array_element)
            (`KismetArrayLibrary.Array_RemoveItem` _actorsingraveyard _array_element)
            (return))))))
  (return))

(fn `RecreateTopGraveyardCardActor`
  (bind _player_index (`self.Player_Index`))
  (bind _graveyardlist (`self.GraveyardList`))
  (bind _returnvalue (`KismetArrayLibrary.Array_LastIndex` _graveyardlist))
  (`/Engine/EditorBlueprintResources/ActorMacros.Switch Has Authority`
    (:`Authority`
      (if (> (`KismetArrayLibrary.Array_Length` (`self.GraveyardList`)) 0)
        (if (== (`KismetArrayLibrary.Array_Length` (`self.ActorsInGraveyard`)) 0)
          (bind _cardcreated (message `/Game/Blueprints/Interface/Controler_interface.CreatePlayableCard` (`/Game/Blueprints/Library/BP_Controler_flib.GetControlerReferenceFromID(serverOnly)` _player_index) (`KismetMathLibrary.Conv_VectorToTransform` (`self.GetCardInGraveyardLocation` 1))))
          (bind _cardref1 (`/Game/Blueprints/Library/BP_Card_flib.SetupCard` _cardcreated _player_index (`|GetArrayItem` _graveyardlist _returnvalue) "NewEnumerator0" (`|GetArrayItem` (`self.GraveyardStructList`) _returnvalue) true))
          (`KismetArrayLibrary.Array_AddUnique` (`self.ActorsInGraveyard`) _cardref1))))))

(fn `RemoveCardFromGraveyard`
  (params (CardName :type Name) (Index :type Integer))
  (bind _actorsingraveyard (`self.ActorsInGraveyard`))
  (bind _output (`|GetArrayItem` _actorsingraveyard))
  (set `self.RemoveIndex` Index)
  (if (and (> (`KismetArrayLibrary.Array_Length` (`self.GraveyardList`)) 0) (== CardName (`|GetArrayItem` (`self.GraveyardList`) (`self.RemoveIndex`))))
    (`KismetArrayLibrary.Array_Remove` (`self.GraveyardStructList`) (`self.RemoveIndex`))
    (`/Engine/EditorBlueprintResources/StandardMacros.IsValid` _output
      (:`Is Valid`
        (`/Game/Blueprints/GamePlay/Locam_3DCard.SetCardHiddenState` _output true)
        (`/Game/Blueprints/GamePlay/Locam_3DCard.RemoveCardActor` _output)
        (`KismetArrayLibrary.Array_Remove` _actorsingraveyard))
      (:`Is Not Valid`
        _))
    (`KismetArrayLibrary.Array_Remove` (`self.GraveyardList`) (`self.RemoveIndex`))))

(fn `ScaleCardGraveyardStaticMesh`
  (bind _sm_graveyard (`self.SM_Graveyard`))
  (bind _returnvalue (`KismetArrayLibrary.Array_Length` (`self.GraveyardList`)))
  (if (> _returnvalue 0)
    (`SceneComponent.SetHiddenInGame` _sm_graveyard false false)
    (else
      (`SceneComponent.SetHiddenInGame` _sm_graveyard true false)))
  (`SceneComponent.K2_SetRelativeLocation` _sm_graveyard (`KismetMathLibrary.MakeVector` 0.0 0.0 (- (* 1.5 (`KismetMathLibrary.Conv_IntToDouble` _returnvalue)) 66.0)) false false)
  (return))

(fn `UserConstructionScript`)