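; Networked 3D card actor for a card game, showing a card's art, stats and keywords and animating its movement.
; Data comes from DT_Cards at construction or a server-side setter that multicasts a refresh, feeding a dynamic front material and text fields.
; PlayMovementAnimation stores a goal that a gated Tick interpolates toward; arrival in the Graveyard state closes the gate and updates the owner's graveyard visual.
; Board placement and MoveCardToGraveyard are empty stubs.
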(event `Multicast_PlaceCardOnBoard`
  (params (Destination :type "Vector Structure") (Rotation :type "Rotator Structure")))

(event `RemoveCardActor`
  ;[0.5469 1 0] Destroy Card
  (`KismetSystemLibrary.Delay` 0.5)
  (`self.K2_DestroyActor`))

(event `Server_SetCardData`
  (params (CardName :type Name) (CardSet :type "/Game/Blueprints/Enums/E_CardSet Enum" :default "NewEnumerator0") (CardStruct :type "/Game/GameRules/Card_Attributes Structure") (SetCardDataFromStruct :type Boolean))
  (`/Engine/EditorBlueprintResources/ActorMacros.Switch Has Authority`
    (:`Authority`
      (`self.SetCardData` CardName CardSet CardStruct SetCardDataFromStruct)
      (`self.Multicast_SetCardVisuals`))))

(event `Multicast_SetCardVisuals`
  (`self.UpdateCardDisplay`))

(event `ForceMoveCardDirectlyToGraveyard`
  (params (Graveyard :type "/Game/Blueprints/GamePlay/GRaveyard Object Reference"))
  (`self.K2_SetActorRotation` (`/Game/Blueprints/Library/BP_flib.GetWorldRotationForPlayer` (struct))))

(event `SetCardHiddenState`
  (params (bNewHidden :type Boolean))
  ;[0.7578 0 1] Multicast - set card hidden
  (`self.SetActorHiddenInGame` bNewHidden)
  (`PrimitiveComponent.SetCollisionEnabled` (`self.CardBase`) "NoCollision"))

(event `self.ReceiveTick`
  (params (DeltaSeconds :type "Float (single-precision)"))
  (bind (_return_value _arrived) (`self.InterpSelfToLocation`))
  (bind (_return_value_2 _arrived_2) (`self.InterpSelfToRotation`))
  ;[1 0 0.6797] Movement Interpolation
  (set `self.DeltaTime` DeltaSeconds)
  (`/Engine/EditorBlueprintResources/StandardMacros.Gate` true :!label _label
    (:`Exit`
      (`self.K2_SetActorTransform` (`KismetMathLibrary.MakeTransform` _return_value _return_value_2))
      (if (and _arrived _arrived_2)
        (`self.ArrivedAtDestination`)))))

(event `ArrivedAtDestination`
  (bind _placementowner (`self.PlacementOwner`))
  (switch `/Game/Blueprints/Enums/E_CardMovementStates` (`self.CardMovementState`)
    (:`NewEnumerator6`
      (`self.CloseGate`)
      (`/Engine/EditorBlueprintResources/StandardMacros.IsValid` _placementowner
        (:`Is Valid`
          (`/Game/Blueprints/GamePlay/GRaveyard.AddToGraeyardVisual` (`/Game/Blueprints/GamePlay/Locam_CardPlacement.Graveyard_ref` _placementowner)))))))

(event `OpenGate`
  ;[1 0 0.6797] Movement Interpolation
  (goto _label :!via `Open`))

(event `CloseGate`
  ;[1 0 0.6797] Movement Interpolation
  (goto _label :!via `Close`))

(fn `InterpSelfToLocation`
  (returns (`Return Value` :type "Vector Structure") (Arrived :type Boolean))
  (bind _goaldestination (`self.GoalDestination`))
  (bind _returnvalue (`self.K2_GetActorLocation` self))
  (bind _returnvalue_2 (`KismetMathLibrary.NearlyEqual_FloatFloat` (`KismetMathLibrary.VSize` (- _returnvalue _goaldestination)) 0.0 (`self.ErrorTolerance`)))
  (return (select `bool` _returnvalue_2 :`false` (`KismetMathLibrary.VInterpTo` _returnvalue _goaldestination (`self.DeltaTime`) (`self.InterpSpeed`)) :`true` _goaldestination) _returnvalue_2))

(fn `InterpSelfToRotation`
  (returns (`Return Value` :type "Rotator Structure") (Arrived :type Boolean))
  (bind _goalrotation (`self.GoalRotation`))
  (bind _returnvalue (`self.K2_GetActorRotation` self))
  (bind _returnvalue_2 (== _returnvalue _goalrotation :`ErrorTolerance` (/ (`self.ErrorTolerance`) 5.0)))
  (return (select `bool` _returnvalue_2 :`false` (`KismetMathLibrary.RInterpTo` _returnvalue _goalrotation (`self.DeltaTime`) (`self.InterpSpeed`)) :`true` _goalrotation) _returnvalue_2))

(fn `MoveCardToGraveyard`)

(fn `OnRep_OwningPlayerID`)

(fn `OnRep_PlacementOwner`)

(fn `PlayMovementAnimation`
  (params (CardMovementState :type "/Game/Blueprints/Enums/E_CardMovementStates Enum" :default "NewEnumerator0") (ManualGoalDestination :type "Vector Structure") (ManualGoalRotation :type "Rotator Structure") (OR_GoalActor :type "Actor Object Reference") (`Z Offset` :type "Float (double-precision)") (ErrorTolerance :type "Float (double-precision)") (InterSpeed :type "Float (double-precision)"))
  (bind (_returnvalue_x _returnvalue_y _returnvalue_z) (`KismetMathLibrary.BreakVector` (`self.K2_GetActorLocation` OR_GoalActor)))
  (set `self.CardMovementState` CardMovementState)
  (`/Engine/EditorBlueprintResources/StandardMacros.IsValid` OR_GoalActor
    (:`Is Valid`
      (set `self.GoalDestination` (`KismetMathLibrary.MakeVector` _returnvalue_x _returnvalue_y (+ _returnvalue_z `Z Offset`)))
      (set `self.GoalRotation` (`self.K2_GetActorRotation` OR_GoalActor)))
    (:`Is Not Valid`
      (set `self.GoalDestination` ManualGoalDestination)
      (set `self.GoalRotation` ManualGoalRotation)))
  (set `self.ErrorTolerance` ErrorTolerance)
  (set `self.InterpSpeed` InterSpeed))

(fn `SetCardData`
  (params (CardDataTableName :type Name) (CardSet :type "/Game/Blueprints/Enums/E_CardSet Enum" :default "NewEnumerator0") (CardStruct :type "/Game/GameRules/Card_Attributes Structure") (SetCardDataFromStruct :type Boolean))
  (if SetCardDataFromStruct
    (set `self.CardAttibutes` CardStruct)
    (else
      (bind _cardstruct (`/Game/Blueprints/Library/BP_Deck_flib.GetCardData` CardDataTableName CardSet))
      (set `self.CardAttibutes` _cardstruct)))
  (set `self.CardDataTableName` CardDataTableName)
  (set `self.CardSet` CardSet)
  (set `self.CardName` (`KismetTextLibrary.Conv_StringToText` (`.Name_2_A41B7DE244194197693687B9317CDF52` (break `/Game/GameRules/Card_Attributes` (`self.CardAttibutes`))))))

(fn `TextFromInt`
  (params (val :type Integer))
  (returns (ReturnValue :type "Text (by ref)"))
  (bind _returnvalue (`KismetTextLibrary.Conv_IntToText` (`KismetMathLibrary.Abs_Int` val)))
  (return (select `int` (+ (`KismetMathLibrary.SignOfInteger` val) 1) :`0` (`|FormatText` "-{val}" _returnvalue) :`1` (`|FormatText` "") :`2` (`|FormatText` "+{val}" _returnvalue))))

(fn `UpdateCardDisplay`
  (bind _materialfront (`self.MaterialFront`))
  (bind (_cardattibutes_name _cardattibutes_image _cardattibutes_description _cardattibutes_cardtype _cardattibutes_manacost _cardattibutes_attack _cardattibutes_defense _cardattibutes_playerhp _cardattibutes_ennemyhp _cardattibutes_carddraw _cardattibutes_breakthrough _cardattibutes_charge _cardattibutes_drain _cardattibutes_guard _cardattibutes_lethal _cardattibutes_ward) (break `/Game/GameRules/Card_Attributes` (`self.CardAttibutes`)))
  (`|ExecutionSequence`
    (:`then_0`
      (`MaterialInstanceDynamic.SetTextureParameterValue` _materialfront "InsideImage" _cardattibutes_image)
      (`MaterialInstanceDynamic.SetScalarParameterValue` _materialfront "CardType" (`KismetMathLibrary.Conv_ByteToDouble` _cardattibutes_cardtype))
      (`MaterialInstanceDynamic.SetScalarParameterValue` _materialfront "PlayerHP" (`KismetMathLibrary.Conv_IntToDouble` _cardattibutes_playerhp))
      (`MaterialInstanceDynamic.SetScalarParameterValue` _materialfront "EnnemyHP" (`KismetMathLibrary.Conv_IntToDouble` _cardattibutes_ennemyhp))
      (`MaterialInstanceDynamic.SetScalarParameterValue` _materialfront "EnnemiHP" (`KismetMathLibrary.Conv_IntToDouble` _cardattibutes_carddraw))
      (`MaterialInstanceDynamic.SetScalarParameterValue` _materialfront "Breakthrough" (`KismetMathLibrary.Conv_BoolToDouble` _cardattibutes_breakthrough))
      (`MaterialInstanceDynamic.SetScalarParameterValue` _materialfront "Charge" (`KismetMathLibrary.Conv_BoolToDouble` _cardattibutes_charge))
      (`MaterialInstanceDynamic.SetScalarParameterValue` _materialfront "Drain" (`KismetMathLibrary.Conv_BoolToDouble` _cardattibutes_drain))
      (`MaterialInstanceDynamic.SetScalarParameterValue` _materialfront "Guard" (`KismetMathLibrary.Conv_BoolToDouble` _cardattibutes_guard))
      (`MaterialInstanceDynamic.SetScalarParameterValue` _materialfront "Lethal" (`KismetMathLibrary.Conv_BoolToDouble` _cardattibutes_lethal))
      (`MaterialInstanceDynamic.SetScalarParameterValue` _materialfront "Ward" (`KismetMathLibrary.Conv_BoolToDouble` _cardattibutes_ward))
      (`MaterialInstanceDynamic.SetScalarParameterValue` _materialfront "InGame" (`KismetMathLibrary.Conv_BoolToDouble` (`self.IsInGame`))))
    (:`then_1`
      (`|ExecutionSequence`
        (:`then_0`
          (`TextRenderComponent.K2_SetText` (`self.ManaCost`) (`KismetTextLibrary.Conv_IntToText` _cardattibutes_manacost)))
        (:`then_1`
          (`TextRenderComponent.K2_SetText` (`self.Attack`) (`KismetTextLibrary.Conv_IntToText` _cardattibutes_attack)))
        (:`then_2`
          (`TextRenderComponent.K2_SetText` (`self.Defense`) (`KismetTextLibrary.Conv_IntToText` _cardattibutes_defense)))
        (:`then_3`
          (`TextRenderComponent.K2_SetText` (`self.PlayerHp`) (`self.TextFromInt` _cardattibutes_playerhp)))
        (:`then_4`
          (`TextRenderComponent.K2_SetText` (`self.EnnemyHp`) (`self.TextFromInt` _cardattibutes_ennemyhp)))
        (:`then_5`
          (`TextRenderComponent.K2_SetText` (`self.DrawCard`) (`self.TextFromInt` _cardattibutes_carddraw)))))))

(fn `UserConstructionScript`
  ;[0.5703 0 1] Create front side material
  (bind _returnvalue (`PrimitiveComponent.CreateDynamicMaterialInstance` (`self.CardBase`) 1 "/Game/Materials/CardFront.CardFront" "None"))
  (set `self.MaterialFront` _returnvalue)
  ;[0.5469 0 1] Get base informations
  (bind _outrownames (`DataTableFunctionLibrary.GetDataTableRowNames` "/Game/GameRules/DT_Cards.DT_Cards"))
  (bind _returnvalue_2 (`|GetDataTableRow` "/Game/GameRules/DT_Cards.DT_Cards" (`|GetArrayItem` _outrownames (`KismetMathLibrary.Conv_ByteToInt` (`self.CardId`))))
    (:`then`
      (set `self.CardAttibutes` _returnvalue_2)
      (`self.UpdateCardDisplay`))))