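; Board placement actor that holds one or several cards for a player in a card game.
; Construction derives fill direction, snaps width, spawns end and centre tile child actors, scales collision and compiles supported card types.
; Add and remove events update the card array and full flag, then multicast every card to its recomputed position and rotation.
; Both spacing helpers that feed this layout are stubs returning zero.
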(event `RemoveCardFrom Placement`
  (params (CardToClear :type "/Game/GameRules/Locam_3DCard Object Reference"))
  (bind _card_array (`self.Card_Array`))
  (`self.RemoveCardFrom Placement` CardToClear)
  (set `self.bIsFull` (>= (`KismetArrayLibrary.Array_Length` (`self.Card_Array`)) (`self.MaxCardsInPlacement`)) :!label _label)
  (for (_array_element _array_index) _card_array
    (bind (_returnvector _returnrotation) (`self.getCardInPlacementLocation` _array_index (`self.MaxCardsInPlacement`) (`KismetArrayLibrary.Array_Length` _card_array)))
    (`/Game/GameRules/Locam_3DCard.Multicast_PlaceCardOnBoard` _array_element _returnvector _returnrotation)))

(event `AddCardToPlacement`
  (params (CardToAdd :type "/Game/GameRules/Locam_3DCard Object Reference"))
  (`KismetArrayLibrary.Array_Add` (`self.Card_Array`) CardToAdd)
  (goto _label))

(fn `CalculateDynamicSpacingLocation`
  (params (Index :type Integer) (MaxCardsInPlacement :type Integer) (CardsInPlacement :type Integer) (CenterOut :type Boolean))
  (returns (ReturnValue :type "Float (double-precision)") (Overlap :type Boolean))
  (return 0.0 false))

(fn `CalculateSpacingLocation`
  (params (Index :type Integer) (MaxCardsInPlacement :type Integer) (CardsInPlacement :type Integer) (Spacing :type "Float (double-precision)"))
  (returns (ReturnValue :type "Float (double-precision)"))
  (return 0.0))

(fn `CompileSupportedCardTypes`
  (bind _bsupportsitems (`self.bSupportsItems`))
  (for _array_element (`|MakeArray` (select `bool` (`self.bSupportsCreature`) :`false` "NewEnumerator4" :`true` "NewEnumerator0" :!type "/Game/GameRules/E_CardType Enum") (select `bool` _bsupportsitems :`false` "NewEnumerator4" :`true` "NewEnumerator1" :!type "/Game/GameRules/E_CardType Enum") (select `bool` _bsupportsitems :`false` "NewEnumerator4" :`true` "NewEnumerator2" :!type "/Game/GameRules/E_CardType Enum") (select `bool` _bsupportsitems :`false` "NewEnumerator4" :`true` "NewEnumerator3" :!type "/Game/GameRules/E_CardType Enum"))
    (`KismetArrayLibrary.Array_Add` (`self.ValidcardTypeArray`) _array_element)))

(fn `CreateVisualBoardTiles`
  (bind _returnvalue (`KismetMathLibrary.FFloor` (`self.PlacementWidth`)))
  (bind _returnvalue_2 (- _returnvalue 1))
  (if (`self.bScaleMulticardPlacement`)
    (for _index (range (+ _returnvalue_2 1))
      (bind _returnvalue_3 (`AddComponent|NODE_AddChildActorComponent-0` :`RelativeTransform` (`KismetMathLibrary.Conv_VectorToTransform` (`KismetMathLibrary.MakeVector` 0.0 (* (- (`KismetMathLibrary.Conv_IntToDouble` _index) (/ (`KismetMathLibrary.Conv_IntToDouble` _returnvalue_2) 2.0)) (`self.CardWidth`))))))
      (`ChildActorComponent.SetChildActorClass` _returnvalue_3 (select `bool` (== _returnvalue 1) :`false` (select `bool` (== _index 0) :`false` (select `bool` (== _returnvalue_2 _index) :`false` (`self.CenterTile`) :`true` (`self.RightEndtile`)) :`true` (`self.LeftEndtile`)) :`true` (`self.SingleTile`))))))

(fn `getCardInPlacementLocation`
  (params (CardIndex :type Integer) (MaxCards :type Integer) (CardsInPlacement :type Integer))
  (returns (returnVector :type "Vector Structure") (returnRotation :type "Rotator Structure"))
  (bind _bmultiplacement (`self.bMultiPlacement`))
  (bind (_returnvalue _overlap) (`self.CalculateDynamicSpacingLocation` CardIndex MaxCards CardsInPlacement (`self.bCenterOut`)))
  (bind _returnvalue_2 (`self.K2_GetActorLocation` self))
  (bind (_returnvalue_roll _returnvalue_pitch _returnvalue_yaw) (`KismetMathLibrary.BreakRotator` (`self.K2_GetActorRotation` self)))
  (bind _returnvalue_3 (* _returnvalue_2 (1.0 1.0 1.0)))
  (bind _returnvalue_4 (select `bool` (`self.bScaleMulticardPlacement`) :`true` (select `bool` (`self.bDynamicSpacing`) :`false` (`self.CalculateSpacingLocation` CardIndex MaxCards CardsInPlacement (`self.CardSpacing`)) :`true` _returnvalue)))
  (bind _returnvalue_5 (select `bool` (and (select `bool` (`self.bDynamicSpacing`) :`false` (<= (`self.CardWidth`) (`self.CardSpacing`)) :`true` _overlap) (>= CardsInPlacement 0)) :`false` 2.0 :!type "Float (single-precision)"))
  (return (`KismetMathLibrary.SelectVector` (+ _returnvalue_3 (0.0 0.0 100.0)) (+ (`KismetMathLibrary.GreaterGreater_VectorRotator` (`KismetMathLibrary.MakeVector` (select `bool` _bmultiplacement :`false` (.x _returnvalue_2)) (select `bool` _bmultiplacement :`false` (.y _returnvalue_2) :`true` (select `bool` (`self.bInvertPlacementDirection`) :`false` _returnvalue_4 :`true` (* _returnvalue_4 -1.0)))) (`self.K2_GetActorRotation` self)) _returnvalue_3) (`self.bMultiPlacement`)) (`KismetMathLibrary.MakeRotator` (+ _returnvalue_roll (select `bool` (`self.bInvertPlacementDirection`) :`false` _returnvalue_5 :`true` (* _returnvalue_5 -1.0))) _returnvalue_pitch _returnvalue_yaw)))

(fn `GetPlacementState`
  (returns (PlayerIndex :type Integer) (bMultiPlacement :type Boolean) (bIsFull :type Boolean) (CardsInPlacement :type Integer) (MaxCardsInPlacement :type Integer) (bSupportsAllCardType :type Boolean) (ValidcardTypeArray :type "Array of /Game/GameRules/E_CardType Enum"))
  (return (`self.PlayerIndex`) (`self.bMultiPlacement`) (`self.bIsFull`) (`KismetArrayLibrary.Array_Length` (`self.Card_Array`)) (`self.MaxCardsInPlacement`) (`self.bSupportsAllCardType`) (`self.ValidcardTypeArray`)))

(fn `RemoveCardFromPlacement`
  (params (`Card to Clear` :type "/Game/GameRules/Locam_3DCard Object Reference"))
  (`KismetArrayLibrary.Array_RemoveItem` (`self.Card_Array`) `Card to Clear`))

(fn `UserConstructionScript`
  (bind _placementwidth (`self.PlacementWidth`))
  (bind _bscalemulticardplacement (`self.bScaleMulticardPlacement`))
  (`|ExecutionSequence`
    (:`then_0`
      ;[0 1 0.6953] Set card Fill Direction
      (switch `/Game/Blueprints/Enums/E_Direction` (`self.FillDirection`)
        (:`NewEnumerator0`
          (set `self.bCenterOut` false)
          (set `self.bInvertPlacementDirection` false))
        (:`NewEnumerator1`
          (set `self.bCenterOut` true)
          (set `self.bInvertPlacementDirection` false))
        (:`NewEnumerator2`
          (set `self.bCenterOut` true)
          (set `self.bInvertPlacementDirection` true))
        (:`NewEnumerator3`
          (set `self.bCenterOut` false)
          (set `self.bInvertPlacementDirection` true))))
    (:`then_1`
      ;[1 0 0.5859] Adapt Placement width
      (set `self.PlacementWidth` (`KismetMathLibrary.FClamp` (`KismetMathLibrary.GridSnap_Float` (`self.PlacementWidth`) 1.0) 1.0 20.0)))
    (:`then_2`
      ;[0 0.2266 1] Set is multicard placement
      (set `self.bMultiPlacement` (> (`self.MaxCardsInPlacement`) 1))
      (`self.CreateVisualBoardTiles`)
      ;[0.03125 1 0] Scaling
      (`SceneComponent.SetWorldScale3D` (`self.PlacementCollision`) (`KismetMathLibrary.MakeVector` 0.0 (+ (select `bool` _bscalemulticardplacement :`false` 160.0 :`true` (* (/ (`KismetMathLibrary.FClamp` (- _placementwidth 1.0) 1.0 _placementwidth) 2.0) (`self.CardWidth`))) (select `bool` _bscalemulticardplacement :`true` (select `bool` (> _placementwidth 1.0) :`true` 160.0 :!type "Float (single-precision)"))))))
    (:`then_3`
      ;[0 0.1797 1] Card types
      (if (`self.bSupportsAllCardType`)
        (set `self.bSupportsCreature` true)
        (set `self.bSupportsItems` true))
      (`self.CompileSupportedCardTypes`))))