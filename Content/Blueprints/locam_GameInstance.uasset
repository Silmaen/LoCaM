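; Game instance that owns the top-level game state and shows or hides the main menu accordingly.
; ShowMainMenu calls MoveToGameState, which skips repeat requests, cleans up the current state via LeaveCurrentState, then switches on the new GameStateE value.
; The main menu widget is created once for the locam human player, cached and added to the viewport, then removed on leaving that state.
; A separate RequestQuit function exits the game.
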(event `ShowMainMenu`
  (`self.MoveToGameState` "NewEnumerator0"))

(fn `DisplayMainMenu`
  ;[0 1 0.1797] Display Main Menu
  (`/Engine/EditorBlueprintResources/StandardMacros.IsValid` (`self.WMainMenu`)
    (:`Is Valid`
      _)
    (:`Is Not Valid`
      (bind _returnvalue (`|CreateWidget` "/Game/Blueprints/Widgets/W_MainMenu.W_MainMenu_C" (`/Game/Blueprints/Library/BP_flib.GetLocamHumanPlayer`)))
      (bind _output_get (set `self.WMainMenu` _returnvalue))))
  (`UserWidget.AddToViewport` _output_get 5))

(fn `MoveToGameState`
  (params (GameMode :type "/Game/Blueprints/Enums/E_GameState Enum" :default "NewEnumerator0"))
  (`self.IsInState?` GameMode
    (:`true`
      (return))
    (:`false`
      (`self.LeaveCurrentState`)
      (bind _output_get (set `self.GameState_e` GameMode))
      (switch `/Game/Blueprints/Enums/E_GameState` _output_get
        (:`NewEnumerator0`
          (`self.DisplayMainMenu`))))))

(fn `requestQuit`
  (`KismetSystemLibrary.QuitGame` null "Quit"))